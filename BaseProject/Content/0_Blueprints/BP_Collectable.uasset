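; BP_Collectable is a pickup item that spins in place and gets absorbed by the player character on overlap.
; On BeginPlay it picks a mesh from its ItemType (battery, or a cube for the propeller cap) and starts a looping timer that rotates it.
; A character entering the Box plays a timeline that shrinks the mesh while pulling it toward the player, then destroys the actor.
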(event OnComponentBeginOverlap(Box)
  (params (OverlappedComponent :type Primitive%20Component%20Object%20Reference) (OtherActor :type Actor%20Object%20Reference) (OtherComp :type Primitive%20Component%20Object%20Reference) (OtherBodyIndex :type Integer) (bFromSweep :type Boolean) (SweepResult :type Hit%20Result%20Structure%20%28by%20ref%29))
  (bind _staticmesh (Variables|Default|GetStaticMesh))
  ;[0.05 0.05 0.05] Pickup
  (Utilities|Casting|CastToUe4ASP_Character OtherActor)
  (bind _newtrack_0 (Timeline|ItemTimeLine Play)
    (:Update
      ;;[0.05 0.05 0.05] Scale Object Down
      (Transformation|SetRelativeScale3D _staticmesh (Math|Vector|Lerp(Vector) "0.300000,0.300000,0.300000" "0, 0, 0" _newtrack_0))
      ;;[0.05 0.05 0.05] Movement Towards Player
      (Transformation|SetWorldLocation _staticmesh (Math|Vector|Lerp(Vector) (Transformation|GetWorldLocation (Variables|Default|GetDefaultSceneRoot)) (Transformation|GetActorLocation OtherActor) _newtrack_0) false false))
    (:Finished
      (Actor|DestroyActor))))

(event Custom|BeginRotation
  ;[0.05 0.05 0.05] Rotation
  (Transformation|AddRelativeRotation (Variables|Default|GetStaticMesh) "0.000000,0.500000, 0" false false))

(event EventBeginPlay
  (Utilities|Time|SetTimerbyEvent (delegate Custom|BeginRotation) 0.01 true)
  ;[0.05 0.05 0.05] Set Mesh
  (Components|StaticMesh|SetStaticMesh (Variables|Default|GetStaticMesh) (Utilities|Select :Index (Variables|Default|GetItemType) :NewEnumerator0 "/Game/5_Meshes/9VBattery.9VBattery" :NewEnumerator1 "/Game/9_Etc/Geometry/Meshes/1M_Cube.1M_Cube")))

(fn ConstructionScript)